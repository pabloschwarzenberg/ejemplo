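; BP_dot is a controllable character with landing animation sync and a lose-life respawn.
; A movement mode change from Falling to Walking clears the IsJumping flag on its AnimBP.
; LooseLife disables input, activates the Explosion component, then after a short delay re-enables input and moves the character to a hardcoded respawn location.
; No life count is tracked here.
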(event Custom|LooseLife
  (Input|DisableInput 0)
  (Components|Activation|Activate (Variables|Default|Getexplosion) true)
  (Utilities|FlowControl|Delay 0.5)
  (Input|EnableInput 0)
  (Transformation|SetActorLocation "-100.000000,160.000000,100.000000" false false))

(event EventBeginPlay)

(event Collision|EventActorBeginOverlap
  (params (OtherActor :type Actor%20Object%20Reference)))

(event EventTick
  (params (DeltaSeconds :type Float%20%28single-precision%29)))

(event EventOnMovementModeChanged
  (params (PrevMovementMode :type EMovementMode%20Enum :default "MOVE_None") (NewMovementMode :type EMovementMode%20Enum :default "MOVE_None") (PrevCustomMode :type Byte :default 0) (NewCustomMode :type Byte :default 0))
  (Utilities|FlowControl|Sequence
    (:then_0
      (if (and (Utilities|Enum|Equal(Enum) PrevMovementMode "MOVE_Falling") (Utilities|Enum|Equal(Enum) NewMovementMode "MOVE_Walking"))
        (Variables|/Script/dot.DotAnimInstance|SetisJumping (Variables|Default|GetanimBP) false)))))

(fn ConstructionScript)